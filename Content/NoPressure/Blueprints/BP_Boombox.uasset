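; BP_Boombox is an interactable boombox actor that toggles music on and off when clicked.
; Hover events switch custom depth and a stencil value on its static mesh, presumably for a highlight effect.
; Clicking flips MusicPlayer's volume multiplier between muted and an audible level rather than stopping playback, and plays a 2D switch sound either way.
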(event EventBeginPlay)

(event Collision|EventActorBeginOverlap
  (params (OtherActor :type Actor%20Object%20Reference)))

(event EventTick
  (params (DeltaSeconds :type Float%20%28single-precision%29)))

(event EventOnUnhover
  (Rendering|SetRenderCustomDepth (Variables|Debug|GetStaticMeshComponent) false))

(event EventOnHover
  (bind _staticmeshcomponent (Variables|Debug|GetStaticMeshComponent))
  (Rendering|SetRenderCustomDepth _staticmeshcomponent true)
  (Rendering|SetCustomDepthStencilValue _staticmeshcomponent 1))

(event EventOnClick
  (bind _musicplayer (Variables|Default|GetMusicPlayer))
  (if (== (Variables|/Script/Engine.AudioComponent|GetVolumeMultiplier (Variables|Default|GetMusicPlayer)) 0.0)
    (Audio|Components|Audio|SetVolumeMultiplier _musicplayer 0.75 :!class /Script/Engine.AudioComponent)
    (Audio|PlaySound2D "/Engine/VREditor/Sounds/UI/Flashlight_Switch.Flashlight_Switch" 1.0 1.5 0.0 0 0)
    (else
      (Audio|Components|Audio|SetVolumeMultiplier _musicplayer 0.0 :!class /Script/Engine.AudioComponent)
      (Audio|PlaySound2D "/Engine/VREditor/Sounds/UI/Flashlight_Switch.Flashlight_Switch" 1.0 1.0 0.0 0 0))))

(fn ConstructionScript)