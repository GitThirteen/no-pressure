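; MeteorSpawner is an actor that repeatedly spawns Meteor actors around its own location, starting on BeginPlay.
; SpawnMeteor re-arms itself with a timer at the SpawnMeteorEvery interval, then spawns a meteor at a random offset in any direction, scaled by up to Variance.
; StartSpawning and StopSpawning toggle the IsSpawning flag, which gates each cycle and ends the timer loop once cleared.
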(event Custom|StartSpawning
  (Variables|Default|SetisSpawning true)
  (CallFunction|SpawnMeteor))

(event Custom|StopSpawning
  (Variables|Default|SetisSpawning false))

(event Custom|SpawnMeteor
  (if (Variables|Default|GetisSpawning)
    (Utilities|Time|SetTimerbyEvent (delegate Custom|SpawnMeteor) (Variables|Default|GetSpawnMeteorEvery))
    (Game|SpawnActorfromClass "/Game/NoPressure/Blueprints/Meteor.Meteor_C" (Math|Transform|MakeTransform (+ (Transformation|GetActorLocation) (* (Math|Random|RandomUnitVector) (* (Math|Random|RandomFloat) (Variables|Default|GetVariance))))) "Undefined" "MultiplyWithRoot" 0 0)))

(event EventBeginPlay
  (CallFunction|StartSpawning))

(event Collision|EventActorBeginOverlap
  (params (OtherActor :type Actor%20Object%20Reference)))

(event EventTick
  (params (DeltaSeconds :type Float%20%28single-precision%29)))

(fn ConstructionScript)