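; CodeBoard is a code puzzle board of nine CodeBoardButton child actors, labelled 1 to 9 on BeginPlay.
; TryWin, which nothing in this graph calls, checks that every button's CurrentState equals its DesiredState.
; When all match, it sets Won and makes Success visible; it never resets either.
; An unconnected debug loop would print each button's label and desired state.
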(event Custom|OnButtonSet
  (params (ButtonChildComp :type Child%20Actor%20Component%20Object%20Reference) (Text :type Text))
  (bind _ascode_board_button (Utilities|Casting|CastToCodeBoardButton (Variables|/Script/Engine.ChildActorComponent|GetChildActor ButtonChildComp)))
  (Rendering|Components|TextRender|SetText (Variables|/Game/NoPressure/Blueprints/CodeBoardButton.CodeBoardButton_C|GetText _ascode_board_button) Text))

(event Custom|TryWin
  (Variables|Default|SetTempWon true)
  (for _array_element (Utilities|Array|MakeArray (Variables|Default|GetButton6) (Variables|Default|GetButton4) (Variables|Default|GetButton3) (Variables|Default|GetButton2) (Variables|Default|GetButton5) (Variables|Default|GetButton1) (Variables|Default|GetButton9) (Variables|Default|GetButton8) (Variables|Default|GetButton7))
    (bind _ascode_board_button (Utilities|Casting|CastToCodeBoardButton (Variables|/Script/Engine.ChildActorComponent|GetChildActor _array_element)))
    (Variables|Default|SetTempWon (and (Variables|Default|GetTempWon) (== (Variables|/Game/NoPressure/Blueprints/CodeBoardButton.CodeBoardButton_C|GetCurrentState _ascode_board_button) (Variables|/Game/NoPressure/Blueprints/CodeBoardButton.CodeBoardButton_C|GetDesiredState _ascode_board_button)))))
  (if (Variables|Default|GetTempWon)
    (Variables|Default|SetWon true)
    (Rendering|SetVisibility (Variables|Default|GetSuccess) true false)))

(event EventBeginPlay
  (CallFunction|OnButtonSet (Variables|Default|GetButton1) "1")
  (CallFunction|OnButtonSet (Variables|Default|GetButton2) "2")
  (CallFunction|OnButtonSet (Variables|Default|GetButton3) "3")
  (CallFunction|OnButtonSet (Variables|Default|GetButton4) "4")
  (CallFunction|OnButtonSet (Variables|Default|GetButton5) "5")
  (CallFunction|OnButtonSet (Variables|Default|GetButton6) "6")
  (CallFunction|OnButtonSet (Variables|Default|GetButton7) "7")
  (CallFunction|OnButtonSet (Variables|Default|GetButton8) "8")
  (CallFunction|OnButtonSet (Variables|Default|GetButton9) "9"))

(event Collision|EventActorBeginOverlap
  (params (OtherActor :type Actor%20Object%20Reference)))

(event EventTick
  (params (DeltaSeconds :type Float%20%28single-precision%29)))

(fn ConstructionScript)