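; BP_CodeBoardTerminal is an interactable terminal that resets the code board when used.
; Hovering outlines or unmarks its Widget component by toggling custom depth rendering with a stencil value.
; Interacting plays a grab haptic on the first player controller, then finds every CodeBoardButton in the level and calls OnReset on each.
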(event EventBeginPlay)

(event Collision|EventActorBeginOverlap
  (params (OtherActor :type Actor%20Object%20Reference)))

(event EventOnInteract
  (params (PlayerPawn :type VR%20Pawn%20Object%20Reference))
  (Class|PlayerController|PlayHapticEffect (Game|GetPlayerController 0) "/Game/NoPressure/Haptics/GrabHapticEffect.GrabHapticEffect" "AnyHand" 1.0 false)
  (bind _outactors (Actor|GetAllActorsOfClass "/Game/NoPressure/Blueprints/CodeBoardButton.CodeBoardButton_C"))
  (for _array_element _outactors
    (Default|OnReset _array_element)))

(event EventTick
  (params (DeltaSeconds :type Float%20%28single-precision%29)))

(event EventOnHover
  (bind _widget (Variables|Default|GetWidget))
  (Rendering|SetRenderCustomDepth _widget true)
  (Rendering|SetCustomDepthStencilValue _widget 1))

(event EventOnUnhover
  (Rendering|SetRenderCustomDepth (Variables|Default|GetWidget) false))

(fn ConstructionScript)