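; AlarmButton is an interactable button that periodically raises a timed alarm the player must switch off.
; A chained timer starts the alarm after a timeout, unpauses its audio and begins a countdown that only prints "DIE" on expiry.
; Interacting during an alarm pauses the audio and reschedules it.
; Tick shows the countdown or an idle message, and hovering outlines the cylinder through custom depth stencil.
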(event Custom|TryStopAlarm
  (if (Variables|Default|GetAlarmOn)
    (Variables|Default|SetAlarmOn false)
    (CallFunction|ScheduleAlarm)))

(event Custom|StartAlarm
  (Variables|Default|SetAlarmOn true)
  (bind _returnvalue (Utilities|Time|SetTimerbyEvent (delegate Custom|ExpireAlarm) (Variables|Default|GetAlarmTime)))
  (Variables|Default|SetAlarmTimer _returnvalue)
  (CallFunction|StartAlarmSound))

(event Custom|ScheduleAlarm
  (bind _returnvalue (Utilities|Time|SetTimerbyEvent (delegate Custom|StartAlarm) (Variables|Default|GetTimeout)))
  (Variables|Default|SetAlarmTimer _returnvalue)
  (CallFunction|StopAlarmSound))

(event Custom|ExpireAlarm
  (Development|PrintString "DIE"))

(event Custom|StartAlarmSound
  (Class|AudioComponent|SetPaused (Variables|Default|GetAudio) false))

(event Custom|StopAlarmSound
  (Class|AudioComponent|SetPaused (Variables|Default|GetAudio) true))

(event EventBeginPlay
  (CallFunction|ScheduleAlarm))

(event Collision|EventActorBeginOverlap
  (params (OtherActor :type Actor%20Object%20Reference)))

(event EventTick
  (params (DeltaSeconds :type Float%20%28single-precision%29))
  (bind _text (Variables|Default|GetText))
  (if (Variables|Default|GetAlarmOn)
    (Rendering|Components|TextRender|SetText _text (|GenerictoText (Math|Float|Ceil (Utilities|Time|GetTimerRemainingTimebyHandle (Variables|Default|GetAlarmTimer)))))
    (else
      (Rendering|Components|TextRender|SetText _text (Variables|Default|GetAlarmMessage)))))

(event EventOnHover
  (Rendering|SetRenderCustomDepth (Variables|Default|GetCylinder) true)
  (Rendering|SetCustomDepthStencilValue (Variables|Default|GetCylinder) 1))

(event EventOnUnhover
  (Rendering|SetRenderCustomDepth (Variables|Default|GetCylinder) false))

(event EventOnInteract
  (params (PlayerPawn :type VR%20Pawn%20Object%20Reference))
  (CallFunction|TryStopAlarm))

(fn ConstructionScript)