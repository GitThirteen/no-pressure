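; BP_FuelCell is a grabbable fuel cell for VR.
; Hovering outlines the Cell mesh through custom depth and stencil.
; Grabbing it marks the owning VRPawn as heavy and enables player input on the actor, and dropping it clears both.
; The interact event is empty.
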(event Custom|OnGrabbed
  (bind _asvrpawn (Utilities|Casting|CastToVRPawn (Components|GetOwner (Variables|/Game/NoPressure/Blueprints/GrabComponent.GrabComponent_C|GetMotionControllerRef (Variables|Default|GetGrabComponent)))))
  (Variables|/Game/NoPressure/Blueprints/VRPawn.VRPawn_C|SetbIsHeavy _asvrpawn true)
  (Input|EnableInput (Game|GetPlayerController 0)))

(event Custom|OnDropped
  (bind _asvrpawn (Utilities|Casting|CastToVRPawn (Components|GetOwner (Variables|/Game/NoPressure/Blueprints/GrabComponent.GrabComponent_C|GetMotionControllerRef (Variables|Default|GetGrabComponent)))))
  (Variables|/Game/NoPressure/Blueprints/VRPawn.VRPawn_C|SetbIsHeavy _asvrpawn false)
  (Input|DisableInput (Game|GetPlayerController 0)))

(event EventBeginPlay)

(event Collision|EventActorBeginOverlap
  (params (OtherActor :type Actor%20Object%20Reference)))

(event EventTick
  (params (DeltaSeconds :type Float%20%28single-precision%29)))

(event EventOnInteract
  (params (PlayerPawn :type VR%20Pawn%20Object%20Reference)))

(event EventOnUnhover
  (Rendering|SetRenderCustomDepth (Variables|Default|GetCell) false))

(event EventOnHover
  (bind _cell (Variables|Default|GetCell))
  (Rendering|SetRenderCustomDepth _cell true)
  (Rendering|SetCustomDepthStencilValue _cell 1))

(fn ConstructionScript)