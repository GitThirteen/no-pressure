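; VRGameMode is the game mode that handles two-player readiness and starts the VR match.
; MarkAsReady stores each player's ready flag, and TryStartGame begins a 15-second countdown when both are ready and two players are on the server.
; A delayed loop sends each count to every VRPawn, halts if readiness is lost, and finally has the authority ServerTravel to SpaceStation.
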(event Custom|TryStartGame
  (if (CallFunction|BothPlayersReady)
    (Variables|Default|SetReadyCountdown 15)
    (Actor|GetAllActorsOfClass "/Game/NoPressure/Blueprints/VRPawn.VRPawn_C" :!label _label)
    (for _array_element 0
      (Default|OnReadyCountdown _array_element (Variables|Default|GetReadyCountdown)))
    (if (CallFunction|BothPlayersReady)
      (if (>= (Variables|Default|GetReadyCountdown) 1)
        (Variables|Default|SetReadyCountdown (- (Variables|Default|GetReadyCountdown) 1))
        (Utilities|FlowControl|Delay 1.0)
        (goto _label)
        (else
          (Development|PrintString "Game Start!")
          (Networking|SwitchHasAuthority
            (:Authority
              (Development|ExecuteConsoleCommand "ServerTravel SpaceStation" 0))))))))

(event Custom|MarkAsReady
  (params (PlayerID :type Integer) (Ready :type Boolean))
  (Utilities|Array|SetArrayElem (Variables|Default|GetReadyStatus) PlayerID Ready))

(event EventBeginPlay)

(event EventTick
  (params (DeltaSeconds :type Float%20%28single-precision%29)))

(fn ConstructionScript)

(fn BothPlayersReady
  (return (Math|Boolean|ANDBoolean (Utilities|Array|Get(acopy) (Variables|Default|GetReadyStatus)) (Utilities|Array|Get(acopy) (Variables|Default|GetReadyStatus) 1) (== (Variables|Default|GetPlayersOnServer) 2))))