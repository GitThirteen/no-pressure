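; Meteor actor that flies toward the MeteorTarget and drops a code digit when shot.
; On BeginPlay it takes its digit text and its blue or orange material from random CodeBoardButton picks, the colour following DesiredState.
; Tick moves it straight at the target at Speed, without sweeping.
; An overlap with a Projectile-tagged component spawns a Digit actor showing that text and destroys the meteor.
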(event OnComponentBeginOverlap(Sphere1)
  (params (OverlappedComponent :type Primitive%20Component%20Object%20Reference) (OtherActor :type Actor%20Object%20Reference) (OtherComp :type Primitive%20Component%20Object%20Reference) (OtherBodyIndex :type Integer) (bFromSweep :type Boolean) (SweepResult :type Hit%20Result%20Structure%20%28by%20ref%29))
  (if (Components|ComponentHasTag OtherComp "Projectile")
    (bind _returnvalue (Game|SpawnActorfromClass "/Game/NoPressure/Blueprints/Digit.Digit_C" (Transformation|GetActorTransform) "Undefined" "MultiplyWithRoot" 0 0))
    (Rendering|Components|TextRender|SetText (Variables|/Game/NoPressure/Blueprints/Digit.Digit_C|GetText _returnvalue) (Variables|Default|GetDigit))
    (Actor|DestroyActor)))

(event EventBeginPlay
  (bind _sphere (Variables|Default|GetSphere))
  (bind _outactors (Actor|GetAllActorsOfClass "/Game/NoPressure/Blueprints/CodeBoardButton.CodeBoardButton_C"))
  (Variables|Default|SetDigit (Variables|/Script/Engine.TextRenderComponent|GetText (Variables|/Game/NoPressure/Blueprints/CodeBoardButton.CodeBoardButton_C|GetText (.OutItem (Utilities|Array|Random _outactors)))))
  (if (Variables|/Game/NoPressure/Blueprints/CodeBoardButton.CodeBoardButton_C|GetDesiredState (.OutItem (Utilities|Array|Random _outactors)))
    (Rendering|Material|SetMaterial _sphere 0 "/Game/NoPressure/Materials/M_SolidBlue.M_SolidBlue")
    (else
      (Rendering|Material|SetMaterial _sphere 0 "/Game/NoPressure/Materials/M_SolidOrange.M_SolidOrange"))))

(event Collision|EventActorBeginOverlap
  (params (OtherActor :type Actor%20Object%20Reference)))

(event EventTick
  (params (DeltaSeconds :type Float%20%28single-precision%29))
  (bind _defaultsceneroot (Variables|Default|GetDefaultSceneRoot))
  (bind _returnvalue (Transformation|GetWorldLocation _defaultsceneroot))
  (bind _returnvalue_2 (Actor|GetActorOfClass "/Game/NoPressure/Blueprints/MeteorTarget.MeteorTarget_C"))
  (Transformation|SetWorldLocation (Variables|Default|GetDefaultSceneRoot) (+ _returnvalue (* (Math|Vector|Normalize (- (Transformation|GetWorldLocation (Variables|/Game/NoPressure/Blueprints/MeteorTarget.MeteorTarget_C|GetDefaultSceneRoot _returnvalue_2)) _returnvalue)) (* DeltaSeconds (Variables|Default|GetSpeed)))) false false))

(fn ConstructionScript)