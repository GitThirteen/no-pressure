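; Two-state puzzle button for the CodeBoard, with randomized desired and current states set on begin play and on reset.
; Interacting flips the current state, then finds the CodeBoard actor by class and calls its TryWin.
; Tick reapplies a blue or orange material every frame to show the current state.
; Hovering toggles custom depth with a stencil value on the button mesh for highlighting.
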(event Custom|OnReset
  (Variables|Default|SetDesiredState (Math|Random|RandomBool))
  (Variables|Default|SetCurrentState (Math|Random|RandomBool)))

(event Custom|OnSwitch
  (Variables|Default|SetCurrentState (not (Variables|Default|GetCurrentState)))
  (bind _returnvalue (Actor|GetActorOfClass "/Game/NoPressure/Blueprints/CodeBoard.CodeBoard_C"))
  (Default|TryWin _returnvalue))

(event EventBeginPlay
  (CallFunction|OnReset))

(event Collision|EventActorBeginOverlap
  (params (OtherActor :type Actor%20Object%20Reference)))

(event EventTick
  (params (DeltaSeconds :type Float%20%28single-precision%29))
  (bind _button (Variables|Default|GetButton))
  (if (Variables|Default|GetCurrentState)
    (Rendering|Material|SetMaterial _button 0 "/Game/NoPressure/Materials/M_SolidBlue.M_SolidBlue")
    (else
      (Rendering|Material|SetMaterial _button 0 "/Game/NoPressure/Materials/M_SolidOrange.M_SolidOrange"))))

(event EventOnHover
  (bind _button (Variables|Default|GetButton))
  (Rendering|SetRenderCustomDepth _button true)
  (Rendering|SetCustomDepthStencilValue _button 1))

(event EventOnUnhover
  (Rendering|SetRenderCustomDepth (Variables|Default|GetButton) false))

(event EventOnInteract
  (params (PlayerPawn :type VR%20Pawn%20Object%20Reference))
  (CallFunction|OnSwitch))

(fn ConstructionScript)