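; BP_SettingsTermiinal is an interactable settings terminal that toggles burst mode on MeteorPistols.
; Hover and unhover switch custom depth rendering on its widget component, using a stencil value for highlighting.
; Interacting plays a grab haptic, then flips BurstMode on every MeteorPistol found in the world.
; The WB_SettingsMenu exit button text is reused to show Burst ON or OFF, based on the looped pistol's state.
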(event EventBeginPlay)

(event Collision|EventActorBeginOverlap
  (params (OtherActor :type Actor%20Object%20Reference)))

(event EventOnInteract
  (params (PlayerPawn :type VR%20Pawn%20Object%20Reference))
  (Class|PlayerController|PlayHapticEffect (Game|GetPlayerController 0) "/Game/NoPressure/Haptics/GrabHapticEffect.GrabHapticEffect" "AnyHand" 1.0 false)
  (bind _outactors (Actor|GetAllActorsOfClass "/Game/NoPressure/Blueprints/MeteorPistol.MeteorPistol_C"))
  (for _array_element _outactors
    (bind _output_get (Variables|/Game/NoPressure/Blueprints/MeteorPistol.MeteorPistol_C|SetBurstMode _array_element (not (Variables|/Game/NoPressure/Blueprints/MeteorPistol.MeteorPistol_C|GetBurstMode _array_element)))))
  (bind _aswb_settings_menu (Utilities|Casting|CastToWB_SettingsMenu (UserInterface|GetWidget (Variables|Default|GetWidget))))
  (if _output_get
    (Rendering|Components|TextRender|SetText (Variables|/Game/NoPressure/Widgets/WB_SettingsMenu.WB_SettingsMenu_C|GetText_ExitButton _aswb_settings_menu) "Burst ON")
    (else
      (Rendering|Components|TextRender|SetText (Variables|/Game/NoPressure/Widgets/WB_SettingsMenu.WB_SettingsMenu_C|GetText_ExitButton _aswb_settings_menu) "Burst OFF"))))

(event EventTick
  (params (DeltaSeconds :type Float%20%28single-precision%29)))

(event EventOnHover
  (bind _widget (Variables|Default|GetWidget))
  (Rendering|SetRenderCustomDepth _widget true)
  (Rendering|SetCustomDepthStencilValue _widget 1))

(event EventOnUnhover
  (Rendering|SetRenderCustomDepth (Variables|Default|GetWidget) false))

(fn ConstructionScript)