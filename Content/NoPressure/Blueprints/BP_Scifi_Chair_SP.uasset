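; BP_Scifi_Chair_SP is an interactable sci-fi chair that a player pawn can sit in and leave.
; Hover toggles a custom depth stencil highlight on the mesh.
; Interacting with a free chair while unseated assigns SeatID to the pawn's PlayerID, saves its transform, makes it immovable and attaches it to SitPos.
; Interacting again from that seat detaches the pawn and restores its transform; any other attempt plays an error sound.
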(event EventBeginPlay)

(event Collision|EventActorBeginOverlap
  (params (OtherActor :type Actor%20Object%20Reference)))

(event EventTick
  (params (DeltaSeconds :type Float%20%28single-precision%29)))

(event EventOnHover
  (bind _staticmeshcomponent (Variables|Debug|GetStaticMeshComponent))
  (Rendering|SetRenderCustomDepth _staticmeshcomponent true)
  (Rendering|SetCustomDepthStencilValue _staticmeshcomponent 1))

(event EventOnUnhover
  (Rendering|SetRenderCustomDepth (Variables|Debug|GetStaticMeshComponent) false))

(event EventOnInteract
  (params (PlayerPawn :type VR%20Pawn%20Object%20Reference))
  (if (and (not (Variables|Default|GetbOccupied)) (== (Variables|/Game/NoPressure/Blueprints/VRPawn.VRPawn_C|GetPlayerID PlayerPawn) -1))
    (Variables|Default|SetPlayerOldTransform (Transformation|GetActorTransform PlayerPawn))
    (Variables|/Game/NoPressure/Blueprints/VRPawn.VRPawn_C|SetPlayerID PlayerPawn (Variables|Default|GetSeatID))
    (Variables|Default|SetbOccupied true)
    (Collision|SetActorEnableCollision PlayerPawn false)
    (Variables|/Game/NoPressure/Blueprints/VRPawn.VRPawn_C|SetbImmovable PlayerPawn true)
    (Transformation|AttachComponentToComponent PlayerPawn (Variables|Default|GetSitPos) "None" "SnapToTarget" "SnapToTarget" "KeepWorld" false)
    (Collision|SetActorEnableCollision PlayerPawn true)
    (elif (== (Variables|/Game/NoPressure/Blueprints/VRPawn.VRPawn_C|GetPlayerID PlayerPawn) (Variables|Default|GetSeatID))
      (Variables|/Game/NoPressure/Blueprints/VRPawn.VRPawn_C|SetPlayerID PlayerPawn -1)
      (Transformation|DetachFromActor PlayerPawn "KeepWorld" "KeepWorld" "KeepWorld")
      (Variables|/Game/NoPressure/Blueprints/VRPawn.VRPawn_C|SetbImmovable PlayerPawn false)
      (Transformation|SetActorTransform PlayerPawn (Variables|Default|GetPlayerOldTransform) false true)
      (Variables|Default|SetbOccupied false)
      (else
        (Audio|PlaySound2D "/Engine/EditorSounds/Notifications/CompileFailed.CompileFailed" 1.0 1.0 0.0 0 0)))))

(fn ConstructionScript)